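; BP_Ai is an enemy AI that wanders, chases nearby third-person characters and damages them at close range.
; A looping timer sends it to random reachable navmesh points through its AIController.
; Tick measures distance to every character, pausing wandering to chase within range; closer still, it calls TakeDamages each tick on the first character found, not necessarily the near one.
; HitAi subtracts Health and destroys the actor at zero.
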(event Custom|Move
  (AI|Navigation|MovetoLocation (stale EventBeginPlay _asaicontroller) (.RandomLocation (AI|Navigation|GetRandomReachablePointinRadius (Transformation|GetActorLocation) 1e+06 (Variables|Default|GetNav%20Data) 0)) -1.0 true true false true 0))

(event EventBeginPlay
  (bind _returnvalue (Actor|GetActorOfClass "/Game/ThirdPerson/Blueprints/BP_ThirdPersonCharacter.BP_ThirdPersonCharacter_C"))
  (Variables|Default|SetPlayerRef _returnvalue)
  (bind _asaicontroller (Utilities|Casting|CastToAIController (Pawn|GetController)))
  (bind _returnvalue_2 (Utilities|Time|SetTimerbyEvent (delegate Custom|Move) 4.0 true))
  (Variables|Default|SetRandomMove _returnvalue_2))

(event EventTick
  (params (DeltaSeconds :type Float%20%28single-precision%29))
  (bind _randommove (Variables|Default|GetRandomMove))
  (bind _outactors (Actor|GetAllActorsOfClass "/Game/ThirdPerson/Blueprints/BP_ThirdPersonCharacter.BP_ThirdPersonCharacter_C"))
  (for _array_element _outactors
    (Utilities|Map|Add (Variables|Default|GetDistanceToAllPlayer) _array_element (Transformation|GetDistanceTo _array_element)))
  (for _array_element_2 _outactors
    (if (<= (.Value (Utilities|Map|Find (Variables|Default|GetDistanceToAllPlayer) _array_element_2)) 4e+02)
      (Utilities|Time|PauseTimerbyHandle _randommove)
      (AI|Navigation|MovetoLocation (stale EventBeginPlay _asaicontroller) (Transformation|GetActorLocation _array_element_2) -1.0 true true false true 0)
      (if (<= (.Value (Utilities|Map|Find (Variables|Default|GetDistanceToAllPlayer) _array_element_2)) 2e+02)
        (bind _returnvalue (Actor|GetActorOfClass "/Game/ThirdPerson/Blueprints/BP_ThirdPersonCharacter.BP_ThirdPersonCharacter_C"))
        (Default|TakeDamages _returnvalue))
      (else
        (Utilities|Time|UnpauseTimerbyHandle _randommove)))))

(fn ConstructionScript)

(fn Death
  (Actor|DestroyActor))

(fn HitAi
  (params (Damage :type Float%20%28double-precision%29))
  (Development|PrintString "Hit")
  (Variables|Default|SetHealth (- (Variables|Default|GetHealth) Damage))
  (if (<= (Variables|Default|GetHealth) 0.0)
    (CallFunction|Death))
  (return))