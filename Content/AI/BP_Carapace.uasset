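; Shell projectile for two-player co-op volleys against BP_Ai, attached to a player's hand until Throw launches it.
; A looping timer redirects it toward the AI closest to P1 when within range.
; Renvoi returns it at the AI after a brief freeze and growing camera shake.
; AI overlaps pause homing, speed it up and bounce it to the other player; enough hits destroy both, with a delayed AI respawn scripted afterward.
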(event OnComponentBeginOverlap(Sphere2)
  (params (OverlappedComponent :type Primitive%20Component%20Object%20Reference) (OtherActor :type Actor%20Object%20Reference) (OtherComp :type Primitive%20Component%20Object%20Reference) (OtherBodyIndex :type Integer) (bFromSweep :type Boolean) (SweepResult :type Hit%20Result%20Structure%20%28by%20ref%29))
  (bind _projectilemovement (Variables|Default|GetProjectileMovement))
  (bind _p1 (Variables|Default|GetP1))
  (bind _aitofocus (Variables|Default|GetAiToFocus))
  (bind _projectilemovement_2 (Variables|Default|GetProjectileMovement))
  ;[1 1 1] Rebond de la carapace sur l'énemie
  (Utilities|Casting|CastToBP_Ai OtherActor)
  (Utilities|Time|PauseTimerbyHandle (Variables|Default|GetHommingRef))
  (Variables|Default|SetSpeed (* 1.2 (Variables|Default|GetSpeed)))
  (switch int (Variables|Default|GetPtoSend)
    (:0
      ;;[1 1 1] GoToP2
      (Variables|/Script/Engine.ProjectileMovementComponent|SetbIsHomingProjectile _projectilemovement false)
      (Variables|/Script/Engine.MovementComponent|SetVelocity _projectilemovement (* (Math|Vector|GetUnitDirection(Vector) (Transformation|GetActorLocation (Variables|Default|GetAiToFocus)) (Transformation|GetActorLocation (Variables|Default|GetP2))) (Variables|Default|GetSpeed))))
    (:1
      ;;[1 1 1] GoToP1
      (Variables|/Script/Engine.ProjectileMovementComponent|SetbIsHomingProjectile _projectilemovement_2 false)
      (Variables|/Script/Engine.MovementComponent|SetVelocity _projectilemovement_2 (* (Math|Vector|GetUnitDirection(Vector) (Transformation|GetActorLocation (Variables|Default|GetAiToFocus)) (Transformation|GetActorLocation (Variables|Default|GetP1))) (Variables|Default|GetSpeed)))))
  (Variables|/Game/AI/BP_Ai.BP_Ai_C|SetNbOfHit _aitofocus (+ (Variables|/Game/AI/BP_Ai.BP_Ai_C|GetNbOfHit _aitofocus) 1))
  (if (== (Variables|/Game/AI/BP_Ai.BP_Ai_C|GetNbOfHit _aitofocus) 5)
    (Default|Destroy (Variables|Default|GetAiToFocus))
    (Actor|DestroyActor)
    (Variables|/Game/ThirdPerson/Blueprints/BP_ThirdPersonCharacter.BP_ThirdPersonCharacter_C|SetHas_A_Carapace _p1 false)
    (Variables|/Game/ThirdPerson/Blueprints/BP_ThirdPersonCharacter.BP_ThirdPersonCharacter_C|SetHas_A_Already_Send _p1 false)
    (Utilities|FlowControl|Delay 3.0)
    (Game|SpawnActorfromClass "/Game/AI/BP_Ai.BP_Ai_C" (Math|Transform|MakeTransform "1680.000000,970.000000,0.062593" "0, 0, 0" "1.000000,1.000000,1.000000") "Undefined" "MultiplyWithRoot" 0 0)))

(event Custom|Throw
  (params (Player :type BP%20Third%20Person%20Character%20Object%20Reference))
  ;[1 1 1] Lancé de la carapace
  ;;[1 1 1] detach actor et envoie vers le devant du perso
  (Transformation|DetachFromActor "KeepWorld" "KeepWorld" "KeepRelative")
  (Variables|/Script/Engine.MovementComponent|SetVelocity (Variables|Default|GetProjectileMovement) (* (Math|Vector|GetUnitDirection(Vector) (Transformation|GetActorLocation Player) (Transformation|GetWorldLocation (Variables|Default|GetArrow))) (Variables|Default|GetSpeed)))
  ;;[1 1 1] Auto corection quand tu est proche
  (bind _returnvalue (Utilities|Time|SetTimerbyEvent (delegate Custom|homming) 0.1 true))
  (Variables|Default|SetHommingRef _returnvalue))

(event Custom|Renvoi
  (params (PlayerToRenvoie :type BP%20Third%20Person%20Character%20Object%20Reference))
  (bind _playerindex (Variables|/Game/ThirdPerson/Blueprints/BP_ThirdPersonCharacter.BP_ThirdPersonCharacter_C|GetPlayerIndex PlayerToRenvoie))
  (bind _returnvalue (Game|GetPlayerController _playerindex))
  ;[1 1 1] Renvoie de la carapace sur l'ai + savoir qui a renvoyer
  ;;[1 1 1] Felling D'arret du mouvement
  (Development|PrintString "Hello")
  (bind _output_get (Variables|Default|SetScale (* (Variables|Default|GetScale) 1.5)))
  (Game|Feedback|ClientStartCameraShake _returnvalue "/Game/AI/ShAKE/Bp_Shake.Bp_Shake_C" _output_get "World" "0, 0, 0")
  (Input|DisableInput PlayerToRenvoie _returnvalue)
  (Components|Movement|StopMovementImmediately (Variables|Default|GetProjectileMovement))
  (Utilities|FlowControl|Delay 0.2)
  (Input|EnableInput PlayerToRenvoie _returnvalue)
  (if (== PlayerToRenvoie (Variables|Default|GetP1))
    (Variables|Default|SetPtoSend 0)
    (else
      (Variables|Default|SetPtoSend 1)))
  (Variables|/Script/Engine.MovementComponent|SetVelocity (Variables|Default|GetProjectileMovement) (* (Math|Vector|GetUnitDirection(Vector) (Transformation|GetActorLocation PlayerToRenvoie) (Transformation|GetActorLocation (Variables|Default|GetAiToFocus))) (Variables|Default|GetSpeed)))
  (Utilities|Time|UnpauseTimerbyHandle (Variables|Default|GetHommingRef)))

(event Custom|homming
  ;[1 1 1] Lancé de la carapace
  ;;[1 1 1] Auto corection quand tu est proche
  (if (<= (Transformation|GetDistanceTo (CallFunction|LessDistanceAi)) 4e+02)
    (Variables|/Script/Engine.MovementComponent|SetVelocity (Variables|Default|GetProjectileMovement) (* (Math|Vector|GetUnitDirection(Vector) (Transformation|GetActorLocation) (Transformation|GetActorLocation (CallFunction|LessDistanceAi))) (Variables|Default|GetSpeed)))))

(event EventBeginPlay
  ;[1 1 1] BeginPlay
  (Utilities|FlowControl|Sequence
    (:then_0
      ;;[1 1 1] Attach carapace au player
      (Utilities|FlowControl|Delay 0.01)
      (Transformation|AttachActorToActor (Variables|Default|GetActorToAttach) "hand_rSocket" "KeepWorld" "KeepWorld" "SnapToTarget" true)
      (Transformation|SetActorLocation (Transformation|GetWorldLocation (Variables|/Game/ThirdPerson/Blueprints/BP_ThirdPersonCharacter.BP_ThirdPersonCharacter_C|GetScene (Variables|Default|GetActorToAttach))) false false))
    (:then_1
      ;;[1 1 1] set les ref
      (bind _returnvalue (Actor|GetActorOfClass "/Game/AI/BP_Ai.BP_Ai_C"))
      (Variables|Default|SetAiRef _returnvalue)
      (bind _outactors (Actor|GetAllActorsOfClass "/Game/ThirdPerson/Blueprints/BP_ThirdPersonCharacter.BP_ThirdPersonCharacter_C"))
      (bind _output_get (Variables|Default|SetP _outactors))
      ;;[1 1 1] Set qui et le p1 et le p2
      (Variables|Default|SetP2 (Utilities|Array|Get(acopy) _output_get (Utilities|Array|LastIndex _output_get)))
      (Variables|Default|SetP1 (Utilities|Array|Get(acopy) (Variables|Default|GetP))))))

(fn ConstructionScript)

(fn LessDistanceAi
  (bind _distance (Variables|Default|GetDistance))
  (bind _outactors (Actor|GetAllActorsOfClass "/Game/AI/BP_Ai.BP_Ai_C"))
  (for _array_element _outactors
    (Utilities|Map|Add (Variables|Default|GetDistance) _array_element (Transformation|GetDistanceTo _array_element (Variables|Default|GetP1))))
  (bind _values (Utilities|Map|Values _distance))
  (bind _keys (Utilities|Map|Keys _distance))
  (Variables|Default|SetAiToFocus (Utilities|Array|Get(acopy) _keys (.IndexOfMinValue (Math|Float|MinOfFloatArray _values))))
  (return (Utilities|Array|Get(acopy) _keys (.IndexOfMinValue (Math|Float|MinOfFloatArray _values)))))